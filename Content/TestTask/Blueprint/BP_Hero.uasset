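; Side-scrolling hero character that runs along Y, turns around, climbs ledges and picks up health potions.
; Jump runs three line traces to find a climbable ledge, then timelines lift the flying hero and, on climb ending, push it forward before restoring walking.
; The VacuumCleaner overlap tracks nearby potions and toggles help text.
; E turns the hero toward the last potion if needed, ramps IK alpha, then destroys it.
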(event OnComponentBeginOverlap(VacuumCleaner)
  (params (OverlappedComponent :type Primitive%20Component%20Object%20Reference) (OtherActor :type Actor%20Object%20Reference) (OtherComp :type Primitive%20Component%20Object%20Reference) (OtherBodyIndex :type Integer) (bFromSweep :type Boolean) (SweepResult :type Hit%20Result%20Structure%20%28by%20ref%29))
  ;[1 1 1] Taking HP
  ;;[1 1 1] Add potions into an array that when they are overlapped with VacuumCleaner
  (bind _asbp_health_pointion (Utilities|Casting|CastToBP_HealthPointion OtherActor))
  (Utilities|Array|Add (Variables|Default|GetHPPotion) _asbp_health_pointion)
  (Utilities|IsValid (Variables|Default|GetUIText)
    (:Is%20Valid
      (Variables|/Game/TestTask/Blueprint/UI_HelpText.UI_HelpText_C|SetTextOpacity (Variables|Default|GetUIText) (Utilities|Struct|MakeSlateColor "(R=1.000000,G=1.000000,B=1.000000,A=1.000000)" "UseColor_Specified")))
    (:Is%20Not%20Valid
      (bind _returnvalue (UserInterface|CreateWidget "/Game/TestTask/Blueprint/UI_HelpText.UI_HelpText_C"))
      (bind _output_get (Variables|Default|SetUIText _returnvalue))
      (UserInterface|Viewport|AddtoViewport _output_get 0))))

(event OnComponentEndOverlap(VacuumCleaner)
  (params (OverlappedComponent :type Primitive%20Component%20Object%20Reference) (OtherActor :type Actor%20Object%20Reference) (OtherComp :type Primitive%20Component%20Object%20Reference) (OtherBodyIndex :type Integer))
  (bind _hppotion (Variables|Default|GetHPPotion))
  ;[1 1 1] Taking HP
  ;;[1 1 1] Delete potions from an array when potions don't overlap more by the sphere
  (bind _asbp_health_pointion (Utilities|Casting|CastToBP_HealthPointion OtherActor))
  (Utilities|Array|RemoveIndex _hppotion (Utilities|Array|FindItem _hppotion _asbp_health_pointion))
  (Utilities|IsValid (Utilities|Array|Get(acopy) _hppotion)
    (:Is%20Not%20Valid
      (Variables|/Game/TestTask/Blueprint/UI_HelpText.UI_HelpText_C|SetTextOpacity (Variables|Default|GetUIText) (Utilities|Struct|MakeSlateColor "(R=1.000000,G=1.000000,B=1.000000,A=0.000000)" "UseColor_Specified")))))

(event Custom|ClimbEnding
  ;[1 1 1] Jump and Climb
  ;;[1 1 1] Custom Event for a Climb Ending notify and launching forward move
  (Variables|Default|SetActorLocation (Transformation|GetActorLocation))
  (bind _speedforward (Timeline|GoForward PlayFromStart)
    (:Update
      (Transformation|SetActorLocation (Math|Vector|Lerp(Vector) (Variables|Default|GetActorLocation) (Math|Vector|MakeVector (.x (Variables|Default|GetActorLocation)) (+ (.y (Variables|Default|GetActorLocation)) (* (Variables|Default|GetCurrentHeroDirection) -1e+02)) (.z (Variables|Default|GetActorLocation))) _speedforward) false false))
    (:Finished
      (Pawn|Components|CharacterMovement|SetMovementMode (Variables|Character|GetCharacterMovement) "MOVE_Walking" 0))))

(event Custom|Turn
  ;[1 1 1] Movement & Turning
  ;;[1 1 1] Turning
  (Variables|Default|SetActorRotateYaw (.yaw (Transformation|GetActorRotation)))
  (Variables|Default|SetTurning true)
  (bind _turning_speed (Timeline|TurningSpeed PlayFromStart)
    (:Update
      (Transformation|SetActorRotation (Math|Rotator|MakeRotator 0.0 0.0 (Math|Float|Lerp (Variables|Default|GetActorRotateYaw) (* (Variables|Default|GetActorRotateYaw) -1.0) _turning_speed))))
    (:Finished
      (Variables|Default|SetTurning false))))

(event EventBeginPlay
  ;[1 1 1] Init
  ;;[1 1 1] Init Climb Animation
  (bind _asbpa_hero (Utilities|Casting|CastToBPA_Hero (Components|SkeletalMesh|GetAnimInstance (Variables|Character|GetMesh))))
  (Variables|Default|SetAnimationRef _asbpa_hero))

(event Input|ActionEvents|InputActionJump
  (params (Key :type Key%20Structure :default "None"))
  ;[1 1 1] Jump and Climb
  (:Pressed
    (bind (_hit _locationwall _heightwall) (CallFunction|ForwardScan))
    (if (Math|Boolean|ANDBoolean _hit (not (Variables|/Game/TestTask/Animation/BPA_Hero.BPA_Hero_C|GetCanClimb (Variables|Default|GetAnimationRef))) (not (AI|Components|NavMovement|IsFalling (Variables|Character|GetCharacterMovement))))
      (bind _output_get (Variables|Default|SetLocationWall _locationwall))
      (bind _output_get_2 (Variables|Default|SetHeightWall _heightwall))
      (Variables|/Game/TestTask/Animation/BPA_Hero.BPA_Hero_C|SetCanClimb (Variables|Default|GetAnimationRef) true)
      (Variables|Default|SetActorLocation (Transformation|GetActorLocation))
      (Pawn|Components|CharacterMovement|SetMovementMode (Variables|Character|GetCharacterMovement) "MOVE_Flying" 0)
      (bind _speed (Timeline|Timeline_0 PlayFromStart)
        (:Update
          (Transformation|SetActorLocation (Math|Vector|Lerp(Vector) (Variables|Default|GetActorLocation) (Math|Vector|MakeVector (.X (Math|Vector|BreakVector _output_get)) (.y (Variables|Default|GetActorLocation)) (+ _output_get_2 77.0)) _speed) false false)))
      (else
        (Character|Jump)))))

(event Input|AxisEvents|InputAxisMoveRight
  (params (AxisValue :type Float%20%28single-precision%29))
  ;[1 1 1] Movement & Turning
  ;;[1 1 1] Movement
  (bind _output_get (Variables|Default|SetHeroDirection AxisValue))
  (if (Math|Boolean|ANDBoolean (!= _output_get 0.0) (not (AI|Components|NavMovement|IsFalling (Variables|Character|GetCharacterMovement))) (not (Variables|Default|GetTurning)) (not (Variables|Default|GetTaking)) (not (Variables|/Game/TestTask/Animation/BPA_Hero.BPA_Hero_C|GetCanClimb (Variables|Default|GetAnimationRef))))
    (if (== (Variables|Default|GetHeroDirection) (Variables|Default|GetCurrentHeroDirection))
      (Pawn|Input|AddMovementInput "0,-1.000000, 0" (Variables|Default|GetHeroDirection) false)
      (else
        (Variables|Default|SetCurrentHeroDirection (Variables|Default|GetHeroDirection))
        (CallFunction|Turn)))))

(event Input|KeyboardEvents|E
  (params (Key :type Key%20Structure :default "None"))
  (bind _hppotion (Variables|Default|GetHPPotion))
  (bind (_object _hppotion_2) (|GetLastHPPotionFromArray _hppotion))
  (bind _returnvalue (Transformation|GetWorldLocation _hppotion_2))
  ;[1 1 1] Taking HP
  (:Pressed
    (Utilities|IsValid (Utilities|Array|Get(acopy) _hppotion)
      (:Is%20Valid
        (if (not (Variables|Default|GetTaking))
          (Variables|Default|SetHPLocation _returnvalue)
          (Variables|Default|SetTaking true)
          (bind _isneedturning (CallFunction|IsNeedTurning _returnvalue))
          (if _isneedturning
            (|TurnHero)
            (bind _alphaspeed (Timeline|IKAlphaSpeed PlayFromStart)
              (:Update
                (Variables|Default|SetIKAlpha _alphaspeed))
              (:Finished
                (Actor|DestroyActor _object)))
            (else
              (Timeline|IKAlphaSpeed PlayFromStart))))))))

(fn ConstructionScript)

(fn ForwardScan
  (bind _returnvalue (Transformation|GetActorLocation))
  (bind _returnvalue_2 (Transformation|GetActorRotation))
  (bind _returnvalue_3 (Transformation|GetActorLocation))
  (bind _returnvalue_4 (Transformation|GetActorLocation))
  (bind _returnvalue_5 (Math|Vector|GetForwardVector _returnvalue_2))
  (bind _returnvalue_6 (+ (.z _returnvalue) 3e+02))
  (bind _returnvalue_7 (* _returnvalue_5 5e+01))
  (bind _returnvalue_8 (Math|Vector|MakeVector (.x _returnvalue) (.y _returnvalue) _returnvalue_6))
  (Utilities|FlowControl|Sequence
    (:then_0
      ;[1 1 1] Check a forward trace
      (bind (_outhit _returnvalue_9) (Collision|LineTraceByChannel _returnvalue_3 (+ _returnvalue_3 (* (Math|Vector|GetForwardVector (Transformation|GetActorRotation)) 75.0)) "TraceTypeQuery3" false 0 "ForDuration" true "(R=1.000000,G=0.000000,B=0.000000,A=1.000000)" "(R=0.000000,G=1.000000,B=0.000000,A=1.000000)" 2.0)))
    (:then_1
      ;[1 1 1] Check a trace from up to down
      (bind (_outhit_2 _returnvalue_10) (Collision|LineTraceByChannel (+ (Math|Vector|MakeVector (.x _returnvalue_4) (.y _returnvalue_4) (+ (.z _returnvalue_4) 3e+02)) _returnvalue_7) (+ _returnvalue_7 (Transformation|GetActorLocation)) "TraceTypeQuery3" false 0 "ForDuration")))
    (:then_2
      (bind _returnvalue_11 (Collision|LineTraceByChannel _returnvalue_8 (+ _returnvalue_8 (* (Math|Vector|GetForwardVector (Transformation|GetActorRotation)) 5e+01)) "TraceTypeQuery3" false 0 "ForDuration" true "(R=1.000000,G=0.000000,B=0.000000,A=1.000000)" "(R=0.000000,G=1.000000,B=0.000000,A=1.000000)" 1e+01)))
    (:then_3
      (return (Math|Boolean|ANDBoolean _returnvalue_9 (and _returnvalue_10 (> (- (.z (.Location (Collision|BreakHitResult _outhit_2))) (+ (.z (Transformation|GetActorLocation)) 1.5e+02)) 0.0)) (not _returnvalue_11)) (.Location (Collision|BreakHitResult _outhit)) (.z (.Location (Collision|BreakHitResult _outhit_2)))))))

(fn IsNeedTurning
  (params (HPLocationF :type Vector))
  (return (and (not (== (Math|Float|Round (.yaw (Transformation|GetActorRotation))) (Math|Float|Round (.yaw (Math|Rotator|FindLookatRotation (Transformation|GetActorLocation) HPLocationF))))) (not (< (Math|Float|Absolute(Float) (- (Math|Float|Absolute(Float) (.y (Transformation|GetActorLocation))) (Math|Float|Absolute(Float) (.Y (Math|Vector|BreakVector HPLocationF))))) 17.0)))))